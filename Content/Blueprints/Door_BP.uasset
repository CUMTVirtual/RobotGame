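; Door actor that swings open and shut in response to open (开门) and close (关门) events, tracking callers with an ActiveButton counter.
; Each open event increments the counter and plays a timeline that lerps the Door component's relative yaw through a quarter turn.
; Each close event decrements the counter and reverses the timeline only at zero, so the door stays open while any activation remains.
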(event `开门`
  (set `self.ActiveButton` (+ (`self.ActiveButton`) 1))
  (bind (_direction `_新建轨道_0`) (`Timeline|时间轴_0` :!label _label)
    (:`Update`
      (`SceneComponent.K2_SetRelativeRotation` (`self.Door`) (`KismetMathLibrary.MakeRotator` 0.0 0.0 (`KismetMathLibrary.Lerp` 0.0 90.0 `_新建轨道_0`)) false false))))

(event `关门`
  (bind _output_get (set `self.ActiveButton` (- (`self.ActiveButton`) 1)))
  (if (== _output_get 0)
    (goto _label :!via `Reverse`)))

(fn `UserConstructionScript`)